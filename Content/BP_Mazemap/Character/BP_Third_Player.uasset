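; Third-person player character holding HP, MP, stamina, EXP and attack/defence stats, with level-up scaling.
; Tick drains stamina while moving, slowing the walk at zero, and regenerates stamina, HP and MP when still.
; Interact, attack and pickup inputs search for the nearest NPC, item or hittable actor and send it interface messages, mostly range-checked.
; Other inputs drive movement, free look, first/third-person camera switching and inventory widget toggling.
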(event EventBeginPlay
  (Utilities|FlowControl|Sequence
    (:then_0
      (CallFunction|InitStat)
      (CallFunction|InitBattleStat))
    (:then_1
      (Input|SetInputModeGameOnly (Game|GetPlayerController 0) false))))

(event EventGetDamaged
  (params (DamageAmouont :type Float%20%28double-precision%29))
  (if (> (Variables|Default|GetPlayerDefenceStat) DamageAmouont)
    (Variables|Default|SetHP (- (Variables|Default|GetHP) 1.0))
    (else
      (Variables|Default|SetHP (+ (- (Variables|Default|GetHP) DamageAmouont) (Variables|Default|GetPlayerDefenceStat)))
      (if (not (> (Variables|Default|GetHP) 0.0))
        (Variables|Default|SetHP 0.0)))))

(event EventGetHP
  (params (HPAmount :type Float%20%28double-precision%29))
  (Variables|Default|SetHP (+ HPAmount (Variables|Default|GetHP)))
  (if (> (Variables|Default|GetHP) (Variables|Default|GetHPMax))
    (Variables|Default|SetHP (Variables|Default|GetHPMax))))

(event EventGetMP
  (params (MPAmount :type Float%20%28double-precision%29))
  (Variables|Default|SetMP (+ MPAmount (Variables|Default|GetMP))))

(event EventGetEXP
  (params (ExpAmount :type Float%20%28double-precision%29))
  (Variables|Default|SetEXP (+ (Variables|Default|GetEXP) ExpAmount))
  (CallFunction|LevelUP))

(event EventTick
  (params (DeltaSeconds :type Float%20%28single-precision%29))
  ;[1 1 1] 스테미나
  (Variables|Default|SetMoving%20Speed (Math|Vector|VectorLength (Variables|/Script/Engine.MovementComponent|GetVelocity (Variables|Character|GetCharacterMovement))))
  (if (== (Variables|Default|GetMoving%20Speed) 0.0)
    (Utilities|FlowControl|Sequence
      (:then_0
        (Variables|/Script/Engine.CharacterMovementComponent|SetMaxWalkSpeed (Variables|Character|GetCharacterMovement) 6e+02)
        (if (>= (Variables|Default|GetStamina) 1e+02)
          (Variables|Default|SetStamina 1e+02)
          (else
            (CallFunction|GetStamina))))
      (:then_1
        (if (<= (Variables|Default|GetHP) (Variables|Default|GetHPMax))
          (CallFunction|StopandHealHP,MP))))
    (else
      (CallFunction|SubStamina))))

(event EventEquipStat
  (params (AttackStat :type Float%20%28double-precision%29) (DefenceStat :type Float%20%28double-precision%29) (SpeedStat :type Float%20%28double-precision%29))
  (Utilities|FlowControl|Sequence
    (:then_0
      (Variables|Default|SetPlayerAttackStat (+ AttackStat (Variables|Default|GetPlayerAttackStat))))
    (:then_1
      (Variables|Default|SetPlayerDefenceStat (+ (Variables|Default|GetPlayerDefenceStat) DefenceStat)))))

(event Input|ActionEvents|InputActionFreeCamera
  (params (Key :type Key%20Structure :default "None"))
  (:Pressed
    (Variables|Default|SetbUseControllerRotationYaw false))
  (:Released
    (Variables|Default|SetbUseControllerRotationYaw true)))

(event Input|ActionEvents|InputActionJump
  (params (Key :type Key%20Structure :default "None"))
  (:Pressed
    (Character|Jump)))

(event Input|ActionEvents|InputActionInteraction(talk)
  (params (Key :type Key%20Structure :default "None"))
  ;[1 1 1] 상호작용
  (:Pressed
    (Development|PrintString "F눌렀음" true true "(R=0.000000,G=0.330729,B=0.036022,A=1.000000)")
    (Utilities|FlowControl|Sequence
      (:then_0
        (bind _outactors (Actor|GetAllActorsOfClass "/Game/BP_Mazemap/Character/NPC/BP_NPC_Parent.BP_NPC_Parent_C"))
        (if (< (.Distance (Actor|FindNearestActor (Transformation|GetActorLocation (Game|GetPlayerCharacter 0)) _outactors)) 2e+02)
          (Class|BPIInteraction|BpiAction(Message) (.ReturnValue (Actor|FindNearestActor (Transformation|GetActorLocation (Game|GetPlayerCharacter 0)) _outactors)) true)))
      (:then_1
        (bind _outactors_2 (Actor|GetAllActorsOfClass "/Game/BP_Mazemap/System/BP_Item_Parent.BP_Item_Parent_C"))
        (if (< (.Distance (Actor|FindNearestActor (Transformation|GetActorLocation (Game|GetPlayerCharacter 0)) _outactors_2)) 2e+02)
          (Class|BPIInteraction|BpiAction(Message) (.ReturnValue (Actor|FindNearestActor (Transformation|GetActorLocation (Game|GetPlayerCharacter 0)) _outactors_2)) true))))))

(event Input|ActionEvents|InputActionPickUp
  (params (Key :type Key%20Structure :default "None"))
  (bind _returnvalue (Game|GetPlayerCharacter 0))
  (bind _returnvalue_2 (Transformation|GetActorLocation _returnvalue))
  ;[1 1 1] 줍기
  (:Released
    (bind _outactors (Actor|GetAllActorsOfClass "/Game/BP_Mazemap/System/BP_Item_Parent.BP_Item_Parent_C"))
    (Class|BPIInteraction|BpiPickup(Message) (.ReturnValue (Actor|FindNearestActor _returnvalue_2 _outactors)) true)
    (if (< (.Distance (Actor|FindNearestActor _returnvalue_2 _outactors)) 1.5e+02)
      (Audio|SpawnSoundatLocation "/Engine/VREditor/Sounds/UI/Object_PickUp.Object_PickUp" _returnvalue_2 "0, 0, 0" 1.0 1.0 0.0 0 0))))

(event Input|ActionEvents|InputActionATtack
  (params (Key :type Key%20Structure :default "None"))
  (:Pressed
    (Development|PrintString "공격" true true "(R=0.705729,G=0.000000,B=0.000000,A=1.000000)")
    (Utilities|FlowControl|Sequence
      (:then_0
        (bind _outactors (Actor|GetAllActorsOfClass "/Game/BP_Mazemap/Character/NPC/BP_NPC_Parent.BP_NPC_Parent_C"))
        (if (< (.Distance (Actor|FindNearestActor (Transformation|GetActorLocation (Game|GetPlayerCharacter 0)) _outactors)) 1e+02)
          (Class|BPIBattle|Attack(Message) (.ReturnValue (Actor|FindNearestActor (Transformation|GetActorLocation (Game|GetPlayerCharacter 0)) _outactors)) (Variables|Default|GetPlayerAttackStat))))
      (:then_1
        (bind _outactors_2 (Actor|GetAllActorsOfClass "/Game/BP_Mazemap/System/BP_CanBeHit_Parent.BP_CanBeHit_Parent_C"))
        (if (< (.Distance (Actor|FindNearestActor (Transformation|GetActorLocation (Game|GetPlayerCharacter 0)) _outactors_2)) 2e+02)
          (Class|BPIBattle|Attack(Message) (.ReturnValue (Actor|FindNearestActor (Transformation|GetActorLocation (Game|GetPlayerCharacter 0)) _outactors_2)) (Variables|Default|GetPlayerAttackStat)))))))

(event Input|ActionEvents|InputActionTransferCamera
  (params (Key :type Key%20Structure :default "None"))
  (:Pressed
    (Utilities|FlowControl|FlipFlop
      (:A
        (Components|Activation|SetActive (Variables|Default|GetFirstPerspectiveCamera) true false)
        (Class|CameraComponent|GetCameraView (Variables|Default|GetFirstPerspectiveCamera) 0.0)
        (Components|Activation|SetActive (Variables|Default|GetCamera) false false))
      (:B
        (Components|Activation|SetActive (Variables|Default|GetCamera) true false)
        (Class|CameraComponent|GetCameraView (Variables|Default|GetCamera) 0.0)
        (Components|Activation|SetActive (Variables|Default|GetFirstPerspectiveCamera) false false)))))

(event Input|ActionEvents|InputActionInventory
  (params (Key :type Key%20Structure :default "None"))
  (:Released
    (Utilities|FlowControl|FlipFlop
      (:A
        (bind _foundwidgets (Widget|GetAllWidgetsOfClass "/Game/BP_Mazemap/System/Widgets/WB_GameWidget.WB_GameWidget_C" true))
        (Class|BPIWidgetSwitch|WidgetInventory(Message) _foundwidgets false))
      (:B
        (bind _foundwidgets_2 (Widget|GetAllWidgetsOfClass "/Game/BP_Mazemap/System/Widgets/WB_GameWidget.WB_GameWidget_C" true))
        (Class|BPIWidgetSwitch|WidgetInventory(Message) _foundwidgets_2 true)))))

(event Input|AxisEvents|InputAxisForward
  (params (AxisValue :type Float%20%28single-precision%29))
  (Pawn|Input|AddMovementInput (Math|Vector|GetForwardVector (Math|Rotator|MakeRotator 0.0 0.0 (.yaw (Pawn|GetControlRotation :!class /Script/Engine.Pawn)))) AxisValue false))

(event Input|AxisEvents|InputAxisRight
  (params (AxisValue :type Float%20%28single-precision%29))
  (Pawn|Input|AddMovementInput (Math|Vector|GetRightVector (Math|Rotator|MakeRotator 0.0 0.0 (.yaw (Pawn|GetControlRotation :!class /Script/Engine.Pawn)))) AxisValue false))

(event Input|AxisEvents|InputAxisSide
  (params (AxisValue :type Float%20%28single-precision%29))
  ;[1 1 1] 코멘트
  (Pawn|Input|AddControllerYawInput AxisValue))

(event Input|AxisEvents|InputAxisLookUp
  (params (AxisValue :type Float%20%28single-precision%29))
  ;[1 1 1] 코멘트
  (Pawn|Input|AddControllerPitchInput AxisValue))

(fn ConstructionScript)

(fn LevelUP
  (if (>= (Variables|Default|GetEXP) (Variables|Default|GetEXPMax))
    (Variables|Default|SetEXP (- (Variables|Default|GetEXP) (Variables|Default|GetEXPMax)))
    (Variables|Default|SetLevel (+ (Variables|Default|GetLevel) 1))
    (Utilities|FlowControl|Sequence
      (:then_0
        (Variables|Default|SetHPMax (* (Variables|Default|GetHPMax) 1.2))
        (Variables|Default|SetPlayerAttackStat (* (Variables|Default|GetPlayerAttackStat) 2.0))
        (Variables|Default|SetPlayerDefenceStat (* (Variables|Default|GetPlayerDefenceStat) 1.5))
        (Variables|Default|SetEXPMax (- (* (Variables|Default|GetEXPMax) 1.4) 3e+01)))
      (:then_1
        (Variables|Default|SetHP (Variables|Default|GetHPMax))
        (Variables|Default|SetMP 1e+02)))))

(fn EXPRate
  (bind _output_get (Variables|Default|SetEXPRate (/ (Variables|Default|GetEXP) (Variables|Default|GetEXPMax))))
  (return _output_get))

(fn HPRate
  (bind _output_get (Variables|Default|SetHPRate (/ (Variables|Default|GetHP) (Variables|Default|GetHPMax))))
  (return _output_get))

(fn GetStamina
  (Utilities|Time|SetTimerbyFunctionName 0 "GetStamina" 3.0)
  (Variables|Default|SetStamina (+ (Variables|Default|GetStamina) 1.0))
  (if (>= 1e+02 (Variables|Default|GetStamina))
    (Class|KismetSystemLibrary|PauseTimer 0 "GetStamina")))

(fn SubStamina
  (Variables|Default|SetStamina (- (Variables|Default|GetStamina) (Variables|Default|GetStamina%20Amount)))
  (if (<= (Variables|Default|GetStamina) 0.0)
    (Variables|Default|SetStamina 0.0)
    (Variables|/Script/Engine.CharacterMovementComponent|SetMaxWalkSpeed (Variables|Character|GetCharacterMovement) 2.5e+02)))

(fn EquipWeapon
  (params (Weapon :type Actor%20Object%20Reference))
  (Transformation|AttachComponentToComponent Weapon (Variables|Character|GetMesh) "gunsocket" "SnapToTarget" "KeepRelative" "KeepWorld" true))

(fn InitStat
  (Variables|Default|SetLevel 1)
  (Utilities|FlowControl|Sequence
    (:then_0
      (Variables|Default|SetEXP (Math|Float|Clamp(Float) 0.0 0.0 (Variables|Default|GetEXPMax)))
      (Variables|Default|SetHP (Math|Float|Clamp(Float) 1e+02 0.0 (Variables|Default|GetHPMax)))
      (Variables|Default|SetMP (Math|Float|Clamp(Float) 1e+02 0.0 1e+02))
      (Variables|Default|SetStamina (Math|Float|Clamp(Float) 1e+02 0.0 1e+02))
      (Variables|Default|SetStamina%20Amount 0.2))
    (:then_1
      (Variables|Default|SetEXPMax 1e+02)
      (Variables|Default|SetHPMax 1e+02))))

(fn InitBattleStat
  (Variables|Default|SetPlayerAttackStat 2e+01)
  (Variables|Default|SetPlayerDefenceStat 35.0))

(fn StopandHealHP,MP
  (Utilities|FlowControl|Sequence
    (:then_0
      (if (>= (Variables|Default|GetHP) (Variables|Default|GetHPMax))
        (Variables|Default|SetHP (Variables|Default|GetHPMax))
        (else
          (Variables|Default|SetHP (+ (Variables|Default|GetHP) 0.7)))))
    (:then_1
      (if (>= (Variables|Default|GetMP) 1e+02)
        (Variables|Default|SetMP 1e+02)
        (else
          (Variables|Default|SetMP (+ (Variables|Default|GetMP) 0.7)))))))