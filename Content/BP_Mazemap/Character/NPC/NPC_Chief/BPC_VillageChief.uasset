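; Village chief NPC that scolds the player as an intruder who sneaked into the village.
; Its BpiAction event prints the accusation on every call, then passes through a DoOnce that prints an order to leave.
; That one-time step also finds BP_Third_Player by class and sends it a monster-attack damage message for 200.
; The second sequence branch does nothing, and construction and BeginPlay only call their parents.
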(event EventBeginPlay
  (|CallParentFunction))

(event Collision|EventActorBeginOverlap
  (params (OtherActor :type Actor%20Object%20Reference))
  (|CallParentFunction OtherActor) ; 지금 이 노드는 비활성 상태입니다. \n핀을 끌어서 다른 노드를 연결하면 활성화됩니다.
)

(event EventTick
  (params (DeltaSeconds :type Float%20%28single-precision%29))
  (|CallParentFunction DeltaSeconds) ; 지금 이 노드는 비활성 상태입니다. \n핀을 끌어서 다른 노드를 연결하면 활성화됩니다.
)

(event EventBpiAction
  (params (Action :type Boolean))
  (Development|PrintString "이놈!! 니가 마을에 몰래 들어온 녀석이냐!")
  (Utilities|FlowControl|Sequence
    (:then_0
      (Utilities|FlowControl|DoOnce false
        (:Completed
          (Development|PrintString "우리 마을에서 꺼져!")
          (bind _returnvalue (Actor|GetActorOfClass "/Game/BP_Mazemap/Character/BP_Third_Player.BP_Third_Player_C"))
          (Class|BPIBattle|PlayerGetDamagedMonsterAttack(Message) _returnvalue 2e+02))))
    (:then_1
      (if true
        _))))

(fn ConstructionScript
  (|CallParentFunction))