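; BPC_Cone is a maze map trap that launches at the player and deals attack damage on contact.
; When the player enters TriggerBox, a timeline moves CapsuleComponent by local offsets without sweep, then hides it.
; Sphere overlap with the player sends AttackDamage to BP_Third_Player and hides the capsule.
; The capsule is only hidden, never destroyed or disabled, and AttackDamage is also passed to InitEnemyStat at BeginPlay.
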(event OnComponentBeginOverlap(TriggerBox)
  (params (OverlappedComponent :type Primitive%20Component%20Object%20Reference) (OtherActor :type Actor%20Object%20Reference) (OtherComp :type Primitive%20Component%20Object%20Reference) (OtherBodyIndex :type Integer) (bFromSweep :type Boolean) (SweepResult :type Hit%20Result%20Structure%20%28by%20ref%29))
  (bind _capsulecomponent (Variables|Default|GetCapsuleComponent))
  (if (== OtherActor (Game|GetPlayerCharacter 0))
    (bind _새_트랙_0 (Timeline|타임라인 Play)
      (:Update
        (Transformation|AddLocalOffset _capsulecomponent _새_트랙_0 false false))
      (:Finished
        (Rendering|SetVisibility _capsulecomponent false false)))))

(event OnComponentBeginOverlap(Sphere)
  (params (OverlappedComponent :type Primitive%20Component%20Object%20Reference) (OtherActor :type Actor%20Object%20Reference) (OtherComp :type Primitive%20Component%20Object%20Reference) (OtherBodyIndex :type Integer) (bFromSweep :type Boolean) (SweepResult :type Hit%20Result%20Structure%20%28by%20ref%29))
  (if (== (Game|GetPlayerCharacter 0) OtherActor)
    (bind _returnvalue (Actor|GetActorOfClass "/Game/BP_Mazemap/Character/BP_Third_Player.BP_Third_Player_C"))
    (Class|BPIBattle|PlayerGetDamagedMonsterAttack(Message) _returnvalue (Variables|Default|GetAttack%20Damage))
    (Rendering|SetVisibility (Variables|Default|GetCapsuleComponent) false false)))

(event EventBeginPlay
  (CallFunction|InitEnemyStat 0 0.0 0.0 0.0 (Variables|Default|GetAttack%20Damage) 0.0))

(event Collision|EventActorBeginOverlap
  (params (OtherActor :type Actor%20Object%20Reference)))

(fn ConstructionScript)

(fn OnMove)