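; BPC_Pool is a maze map pool that heals the player character when it overlaps the pool's static mesh.
; The overlap calls Heal, which sets a looping timer on itself and sends the heal amount to BP_Third_Player through PlayerGetHPMessage.
; The timer pauses when either HP reaches its maximum or stamina reaches its threshold.
; No end-overlap handler exists, so leaving the pool does not stop the healing.
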(event OnComponentBeginOverlap(StaticMesh)
  (params (OverlappedComponent :type Primitive%20Component%20Object%20Reference) (OtherActor :type Actor%20Object%20Reference) (OtherComp :type Primitive%20Component%20Object%20Reference) (OtherBodyIndex :type Integer) (bFromSweep :type Boolean) (SweepResult :type Hit%20Result%20Structure%20%28by%20ref%29))
  (if (== (Game|GetPlayerCharacter 0) OtherActor)
    (CallFunction|Heal)))

(event EventBeginPlay
  (|CallParentFunction)
  (Variables|Default|SetHealAmount 2e+01))

(event Collision|EventActorBeginOverlap
  (params (OtherActor :type Actor%20Object%20Reference))
  (|CallParentFunction OtherActor) ; 지금 이 노드는 비활성 상태입니다. \n핀을 끌어서 다른 노드를 연결하면 활성화됩니다.
)

(event EventTick
  (params (DeltaSeconds :type Float%20%28single-precision%29))
  (|CallParentFunction DeltaSeconds) ; 지금 이 노드는 비활성 상태입니다. \n핀을 끌어서 다른 노드를 연결하면 활성화됩니다.
)

(fn ConstructionScript
  (|CallParentFunction))

(fn Heal
  (Utilities|Time|SetTimerbyFunctionName 0 "Heal" 0.6 true)
  (bind _returnvalue (Actor|GetActorOfClass "/Game/BP_Mazemap/Character/BP_Third_Player.BP_Third_Player_C"))
  (Class|BPIBattle|PlayerGetHP(Message) _returnvalue (Variables|Default|GetHealAmount))
  (Utilities|FlowControl|Sequence
    (:then_0
      (if (>= (Variables|/Game/BP_Mazemap/Character/BP_Third_Player.BP_Third_Player_C|GetHP _returnvalue) (Variables|/Game/BP_Mazemap/Character/BP_Third_Player.BP_Third_Player_C|GetHPMax _returnvalue))
        (Class|KismetSystemLibrary|PauseTimer 0 "Heal" :!label _label)))
    (:then_1
      (if (>= (Variables|/Game/BP_Mazemap/Character/BP_Third_Player.BP_Third_Player_C|GetStamina _returnvalue) 1e+02)
        (goto _label)))))