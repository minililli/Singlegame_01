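; Banana tree quest actor for the maze map that drops up to three bananas when attacked.
; Each Attack clears the next banana flag and spawns a BP_Banana at a random Y offset from the tree.
; The daylight interface restores all flags when Morning is false and the tree is empty.
; Mesh visibility follows the flags only at BeginPlay; an older timeline-based falling animation is left unconnected.
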(event EventBeginPlay
  (Rendering|SetVisibility (Variables|Default|GetBananaMesh1) (Variables|Default|GetBN1%20Visible) false)
  (Rendering|SetVisibility (Variables|Default|GetBananaMesh2) (Variables|Default|GetBN2%20Visible) false)
  (Rendering|SetVisibility (Variables|Default|GetBananaMesh3) (Variables|Default|GetBN3%20Visible) false))

(event EventAttack
  (params (AttackAmount :type Float%20%28double-precision%29))
  (Development|PrintString "맞음ㅇㅇ")
  (if (Variables|Default|GetBN1%20Visible)
    (Variables|Default|SetBN1%20Visible false)
    (Development|PrintString "없어져라 바나나야")
    (CallFunction|BananaSpawn)
    (elif (Variables|Default|GetBN2%20Visible)
      (Variables|Default|SetBN2%20Visible false)
      (CallFunction|BananaSpawn)
      (elif (Variables|Default|GetBN3%20Visible)
        (Variables|Default|SetBN3%20Visible false)
        (CallFunction|BananaSpawn)))))

(event EventBpiDaylight
  (params (Morning :type Boolean))
  (if (not Morning)
    (if (not (Variables|Default|GetBN3%20Visible))
      (Variables|Default|SetBN1%20Visible true)
      (Variables|Default|SetBN2%20Visible true)
      (Variables|Default|SetBN3%20Visible true))))

(fn ConstructionScript)

(fn BananaSpawn
  (bind _returnvalue (Transformation|GetActorLocation))
  (Game|SpawnActorfromClass "/Game/BP_Mazemap/Quest/02-BananaTree/BP_Banana.BP_Banana_C" (Math|Transform|MakeTransform (Math|Vector|MakeVector (.x _returnvalue) (- (.y _returnvalue) (Math|Random|RandomFloatinRange 5e+01 1e+02)) 0.0) "0, 0, 0" "1.000000,1.000000,1.000000") "AdjustIfPossibleButAlwaysSpawn" 0 0)
  (Development|PrintString "바나나소환함" true true "(R=0.705729,G=0.000000,B=0.000000,A=1.000000)"))