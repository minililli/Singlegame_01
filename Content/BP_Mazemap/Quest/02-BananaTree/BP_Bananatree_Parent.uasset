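; Parent Blueprint for quest banana trees that drop bananas when attacked.
; Each Attack plays a timeline dropping TimelineBanana3, then resetting and hiding it, while hiding the next visible banana mesh and spawning a randomly offset BP_Banana.
; The last banana also turns off the tree light.
; Non-morning BpiDaylight events restore visibility only if BananaMesh3 is still visible, so emptied trees stay bare; older per-banana fall logic is unconnected.
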(event EventBeginPlay
  (Variables|Default|SetTLBanana%20Init%20Location (Transformation|GetWorldLocation (Variables|Rendering|GetTimelineBanana3)))
  (Rendering|SetVisibility (Variables|Default|GetTreeBanana) true false))

(event EventAttack
  (params (AttackAmount :type Float%20%28double-precision%29))
  (bind _bananamesh1 (Variables|Default|GetBananaMesh1))
  (bind _bananamesh2 (Variables|Default|GetBananaMesh2))
  (bind _bananamesh3 (Variables|Default|GetBananaMesh3))
  (Utilities|FlowControl|Sequence
    (:then_0
      (bind _fall (Timeline|BananaFall Play)
        (:Update
          (Transformation|AddLocalOffset (Variables|Rendering|GetTimelineBanana3) (Math|Vector|MakeVector 0.0 0.0 (.z _fall)) false false))
        (:Finished
          (Transformation|SetWorldLocation (Variables|Rendering|GetTimelineBanana3) (Variables|Default|GetTLBanana%20Init%20Location) false false)
          (Rendering|SetVisibility (Variables|Rendering|GetTimelineBanana3) false false))))
    (:then_1
      (if (Rendering|IsVisible (Variables|Default|GetBananaMesh1))
        (CallFunction|BananaSpawn _bananamesh1)
        (Rendering|SetVisibility _bananamesh1 false false)
        (elif (Rendering|IsVisible (Variables|Default|GetBananaMesh2))
          (CallFunction|BananaSpawn _bananamesh2)
          (Rendering|SetVisibility _bananamesh2 false false)
          (elif (Rendering|IsVisible (Variables|Default|GetBananaMesh3))
            (CallFunction|BananaSpawn _bananamesh3)
            (Rendering|SetVisibility _bananamesh3 false false)))))))

(event EventBpiDaylight
  (params (Morning :type Boolean))
  ;[1 1 1] 밤마다 바나나 생성이 안됨
  (if (not Morning)
    (if (Rendering|IsVisible (Variables|Default|GetBananaMesh3))
      (Rendering|SetVisibility (Variables|Rendering|GetTimelineBanana3) true false))))

(fn ConstructionScript)

(fn BananaSpawn
  (params (Visibility%20Target :type Static%20Mesh%20Component%20Object%20Reference))
  (bind _returnvalue (Math|Random|RandomFloatinRange -1e+02 1e+02))
  (bind _returnvalue_2 (Transformation|GetActorLocation))
  (Game|SpawnActorfromClass "/Game/BP_Mazemap/Quest/02-BananaTree/BP_Banana.BP_Banana_C" (Math|Transform|MakeTransform (Math|Vector|MakeVector (- (.x _returnvalue_2) _returnvalue) (- (.y _returnvalue_2) _returnvalue) 0.0) (Math|Rotator|MakeRotator 0.0 0.0 (Math|Random|RandomFloatinRange -9e+01 1.8e+02)) "1.000000,1.000000,1.000000") "AdjustIfPossibleButAlwaysSpawn" 0 0)
  (Development|PrintString "바나나소환함" true true "(R=0.000000,G=0.330729,B=0.036022,A=1.000000)"))