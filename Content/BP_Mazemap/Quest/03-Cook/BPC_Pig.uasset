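; BPC_Pig is a pig enemy for the cooking quest that sets its level, health, damage, defence and EXP reward on BeginPlay and shows its name and level.
; Attacks subtract damage above Defence, or a single point when the attack is weaker.
; At zero HP it is destroyed and awards EXP to the player found via GetActorOfClass.
; The daylight interface event, noted for morning spawning, is still empty.
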(event EventBeginPlay
  (|CallParentFunction)
  (CallFunction|InitEnemyStat 2 5e+01 2e+01 45.0 1e+01 5.0)
  (Variables|Default|SetId_Name "PIG")
  (Rendering|Components|TextRender|SetText (Variables|Default|GetName) (Variables|Default|GetId_Name))
  (Rendering|Components|TextRender|SetText (Variables|Default|GetRealLevel) (Utilities|Text|ToText(String) (Variables|Default|GetLevel_0))))

(event Collision|EventActorBeginOverlap
  (params (OtherActor :type Actor%20Object%20Reference))
  (|CallParentFunction OtherActor) ; 지금 이 노드는 비활성 상태입니다. \n핀을 끌어서 다른 노드를 연결하면 활성화됩니다.
)

(event EventTick
  (params (DeltaSeconds :type Float%20%28single-precision%29))
  (|CallParentFunction DeltaSeconds))

(event EventBpiDaylight
  (params (Morning :type Boolean))
  ;[1 1 1] 아침이 되면 생기게 하기
  (if Morning
    _))

(event EventAttack
  (params (AttackAmount :type Float%20%28double-precision%29))
  (CallFunction|GetDamage AttackAmount)
  (if (not (> (Variables|Default|GetHP_0) 0.0))
    (Variables|Default|SetHP_0 0.0)
    (Actor|DestroyActor)
    (bind _returnvalue (Actor|GetActorOfClass "/Game/BP_Mazemap/Character/BP_Third_Player.BP_Third_Player_C"))
    (Class|BPIBattle|GetEXP(Message) _returnvalue (Variables|Default|GetGive%20EXP))))

(fn ConstructionScript
  (|CallParentFunction))

(fn GetDamage
  (params (AttackAmount :type Float%20%28double-precision%29))
  (if (< AttackAmount (Variables|Default|GetDefence_0))
    (Variables|Default|SetHP_0 (- (Variables|Default|GetHP_0) 1.0))
    (else
      (Variables|Default|SetHP_0 (- (Variables|Default|GetHP_0) (- AttackAmount (Variables|Default|GetDefence_0))))))
  (return 0.0))