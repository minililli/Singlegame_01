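; Wolf enemy for the Cook quest in the maze map, which fights by counterattacking the player.
; BeginPlay passes its level, health, mana, EXP reward, attack and defence values to InitEnemyStat.
; The Attack event subtracts defence from incoming damage, or removes 1 HP when defence fully covers the hit.
; At zero HP it destroys itself; otherwise AttackPlayer sends its damage to the player character through AttackMessage.
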(event EventBeginPlay
  (|CallParentFunction)
  (CallFunction|InitEnemyStat (Variables|Default|GetLevel_0) (Variables|Default|GetHP_0) (Variables|Default|GetMP_0) (Variables|Default|GetGive%20EXP) (Variables|Default|GetAttack%20Damage) (Variables|Default|GetDefence_0)))

(event Collision|EventActorBeginOverlap
  (params (OtherActor :type Actor%20Object%20Reference))
  (|CallParentFunction OtherActor) ; 지금 이 노드는 비활성 상태입니다. \n핀을 끌어서 다른 노드를 연결하면 활성화됩니다.
)

(event EventTick
  (params (DeltaSeconds :type Float%20%28single-precision%29))
  (|CallParentFunction DeltaSeconds) ; 지금 이 노드는 비활성 상태입니다. \n핀을 끌어서 다른 노드를 연결하면 활성화됩니다.
)

(event EventAttack
  (params (AttackAmount :type Float%20%28double-precision%29))
  (if (>= (Variables|Default|GetDefence_0) AttackAmount)
    (Variables|Default|SetHP_0 (- (Variables|Default|GetHP_0) 1.0))
    (else
      (bind _output_get (Variables|Default|SetHP_0 (+ (- (Variables|Default|GetHP_0) AttackAmount) (Variables|Default|GetDefence_0))))
      (Development|PrintString (Utilities|String|ToString(Float) _output_get))))
  (if (<= (Variables|Default|GetHP_0) 0.0)
    (Variables|Default|SetHP_0 0.0)
    (Actor|DestroyActor)
    (else
      (CallFunction|AttackPlayer))))

(fn ConstructionScript
  (|CallParentFunction))

(fn AttackPlayer
  (Class|BPIBattle|Attack(Message) (Game|GetPlayerCharacter 0) (Variables|Default|GetAttack%20Damage)))