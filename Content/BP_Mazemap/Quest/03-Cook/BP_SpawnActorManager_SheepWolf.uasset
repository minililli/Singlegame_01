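; Spawn manager that swaps the map's animals by time of day, with sheep in the morning and wolves otherwise.
; It reacts to the BpiDaylight event, destroying all animals of the opposite type and resetting their spawn counter.
; Each call spawns one animal through a capped DoN, at random X/Y within the manager's bounds with random yaw.
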(event EventBeginPlay)

(event Collision|EventActorBeginOverlap
  (params (OtherActor :type Actor%20Object%20Reference)))

(event EventTick
  (params (DeltaSeconds :type Float%20%28single-precision%29)))

(event EventBpiDaylight
  (params (Morning :type Boolean))
  (bind (_origin _boxextent) (Collision|GetActorBounds false false))
  (bind (_origin_2 _boxextent_2) (Collision|GetActorBounds false false))
  (bind _returnvalue (Math|Random|RandomPointinBoundingBox _origin _boxextent))
  (bind _returnvalue_2 (Math|Random|RandomPointinBoundingBox _origin_2 _boxextent_2))
  (if Morning
    (Utilities|FlowControl|Sequence
      (:then_0
        (Utilities|FlowControl|DoN 30 :!label _label
          (:Exit
            (Game|SpawnActorfromClass "/Game/BP_Mazemap/Quest/03-Cook/Sheep/BPC_Sheep.BPC_Sheep_C" (Math|Transform|MakeTransform (Math|Vector|MakeVector (.x _returnvalue) (.y _returnvalue) 0.0) (Math|Rotator|MakeRotator 0.0 0.0 (Math|Random|RandomFloatinRange -1.8e+02 1.8e+02)) "1.000000,1.000000,1.000000") "AdjustIfPossibleButAlwaysSpawn" 0 0.0 0.0 1 0.0 0.0 0.0 0))))
      (:then_1
        (bind _outactors (Actor|GetAllActorsOfClass "/Game/BP_Mazemap/Quest/03-Cook/BPC_Wolf.BPC_Wolf_C"))
        (for _array_element _outactors
          (Actor|DestroyActor _array_element)))
      (:then_2
        (goto _label_2 Reset)))
    (else
      (Utilities|FlowControl|Sequence
        (:then_0
          (goto _label Reset))
        (:then_1
          (Utilities|FlowControl|DoN 15 :!label _label_2
            (:Exit
              (Game|SpawnActorfromClass "/Game/BP_Mazemap/Quest/03-Cook/BPC_Wolf.BPC_Wolf_C" (Math|Transform|MakeTransform (Math|Vector|MakeVector (.x _returnvalue_2) (.y _returnvalue_2) 0.0) (Math|Rotator|MakeRotator 0.0 0.0 (Math|Random|RandomFloatinRange -1.8e+02 1.8e+02)) "1.000000,1.000000,1.000000") "AdjustIfPossibleButAlwaysSpawn" 0 0.0 0.0 1 0.0 0.0 0.0 0))))
        (:then_2
          (bind _outactors_2 (Actor|GetAllActorsOfClass "/Game/BP_Mazemap/Quest/03-Cook/Sheep/BPC_Sheep.BPC_Sheep_C"))
          (for _array_element_2 _outactors_2
            (Actor|DestroyActor _array_element_2)))))))

(fn ConstructionScript)