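; BPC_Sheep is a damageable sheep in the Cook quest, built as a child Blueprint that inherits its enemy stat setup.
; Attack subtracts the amount from HP, prints the result and destroys the actor at zero or below.
; The printed name comes from GetActorOfClass, so it may belong to another sheep.
; Releasing PickUp only prints a debug message, and BpiAction is empty.
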(event EventBeginPlay)

(event Collision|EventActorBeginOverlap
  (params (OtherActor :type Actor%20Object%20Reference)))

(event EventTick
  (params (DeltaSeconds :type Float%20%28single-precision%29)))

(event EventAttack
  (params (AttackAmount :type Float%20%28double-precision%29))
  (bind _output_get (Variables|Default|SetHP (- (Variables|Default|GetHP) AttackAmount)))
  (bind _returnvalue (Actor|GetActorOfClass "BPC_Sheep_C"))
  (Development|PrintString (Utilities|String|Append (Utilities|GetDisplayName _returnvalue) "HP : " (Utilities|String|ToString(Float) _output_get)))
  (if (<= _output_get 0.0)
    (Actor|DestroyActor)))

(event EventBpiAction
  (params (Action :type Boolean)))

(event Input|ActionEvents|InputActionPickUp
  (params (Key :type Key%20Structure))
  (:Released
    (Development|PrintString "줏음")))

(fn ConstructionScript
  (|CallParentFunction))

(fn InitEnemyStat
  (|CallParentFunction))