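; BP_Item_Parent is a base actor for items that shows a pickup prompt when the player comes near.
; Sphere overlaps send interaction-range interface messages; the enter event attaches a screen-space WB_PickUp widget above the item and disables Sphere collision.
; The exit event only prints, leaving widget cleanup logic unconnected.
; Cursor hover events print placeholder text for an item description, and the category switch on BeginPlay has empty branches.
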(event OnComponentBeginOverlap(Sphere)
  (params (OverlappedComponent :type Primitive%20Component%20Object%20Reference) (OtherActor :type Actor%20Object%20Reference) (OtherComp :type Primitive%20Component%20Object%20Reference) (OtherBodyIndex :type Integer) (bFromSweep :type Boolean) (SweepResult :type Hit%20Result%20Structure%20%28by%20ref%29))
  (if (== OtherActor (Game|GetPlayerCharacter 0))
    (Class|BPIInteraction|BpiWBInteractionRangeEnter(Message) self)))

(event OnComponentEndOverlap(Sphere)
  (params (OverlappedComponent :type Primitive%20Component%20Object%20Reference) (OtherActor :type Actor%20Object%20Reference) (OtherComp :type Primitive%20Component%20Object%20Reference) (OtherBodyIndex :type Integer))
  (if (== (Game|GetPlayerCharacter 0) OtherActor)
    (Class|BPIInteraction|BpiWBInteractionRangeExit(Message) self)))

(event Custom|OnBeginCursorOver_Event
  (params (TouchedActor :type Actor%20Object%20Reference))
  (Development|PrintString "아이템 설명 뿅"))

(event Custom|OnEndCursorOver_Event
  (params (TouchedActor :type Actor%20Object%20Reference))
  (Development|PrintString "아이템  설명 닫기"))

(event EventBeginPlay
  (Utilities|FlowControl|Sequence
    (:then_0
      (switch Utilities|FlowControl|Switch|SwitchonEn_ItemCategories (Variables|Default|GetEn_ItemCategory)))
    (:then_1
      (EventDispatchers|BindEventtoOnBeginCursorOver (delegate Custom|OnBeginCursorOver_Event)))
    (:then_2
      (EventDispatchers|BindEventtoOnEndCursorOver (delegate Custom|OnEndCursorOver_Event)))))

(event Collision|EventActorBeginOverlap
  (params (OtherActor :type Actor%20Object%20Reference)))

(event EventTick
  (params (DeltaSeconds :type Float%20%28single-precision%29)))

(event EventBpiWBInteractionRangeEnter
  (bind _returnvalue (UserInterface|CreateWidget "/Game/BP_Mazemap/System/Widgets/WB_PickUp.WB_PickUp_C" (Game|GetPlayerController 0)))
  (bind _returnvalue_2 (AddComponent|AddWidgetComponent false (Math|Transform|MakeTransform "0.000000,0.000000,150.000000" (Pawn|GetControlRotation (Game|GetPlayerCharacter 0) :!class /Script/Engine.Pawn) "1.000000,1.000000,1.000000")))
  (bind _output_get (Variables|Default|SetInteractionWidgetComponent _returnvalue_2))
  (UserInterface|SetWidget _output_get _returnvalue)
  (Class|WidgetComponent|SetWidgetSpace _output_get "Screen")
  (Class|WidgetComponent|SetDrawatDesiredSize _output_get true)
  (Collision|SetCollisionEnabled (Variables|Default|GetSphere) "NoCollision")
  (Transformation|AttachComponentToComponent _output_get (Variables|Default|GetSphere) "None" "KeepRelative" "KeepRelative" "KeepRelative" true))

(event EventBpiWBInteractionRangeExit
  (Development|PrintString "나감"))

(fn ConstructionScript)

(fn Enum
  (params (NewParam :type Boolean)))