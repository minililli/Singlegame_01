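; Light manager that runs a day/night cycle for the maze map by slowly rotating the level's directional light.
; Each Tick fetches the light, nudges its rotation by a fixed, frame-rate-dependent step and derives a Daytime flag from its pitch sign.
; That flag is broadcast every frame to all MovingWall_01_Rotate actors through BpiDaylightMessage.
; A counter-based alternative and debug prints remain disconnected.
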(event Collision|EventActorBeginOverlap
  (params (OtherActor :type Actor%20Object%20Reference)))

(event EventTick
  (params (DeltaSeconds :type Float%20%28single-precision%29))
  (CallFunction|MoringNightTime))

(event EventBeginPlay
  (Variables|Default|SetDaytime (< (.pitch (Variables|Default|GetDL_Init%20Rotation%20Vector)) 0.0)))

(fn ConstructionScript)

(fn MoringNightTime
  (bind _returnvalue (Actor|GetActorOfClass "/Script/Engine.DirectionalLight"))
  (bind _output_get (Variables|Default|SetActor_DirectionalLight _returnvalue))
  (Transformation|AddLocalRotation (Variables|/Script/Engine.Actor|GetRootComponent _output_get) "0.050000,0.000000,0.000000" false false)
  (if (> (.Pitch (Math|Rotator|BreakRotator (Transformation|GetActorRotation (Variables|Default|GetActor_DirectionalLight)))) 0.0)
    (Variables|Default|SetDaytime false)
    (else
      (Variables|Default|SetDaytime true)))
  (bind _outactors (Actor|GetAllActorsOfClass "/Game/BP_Mazemap/MAP/MovingWall_01_Rotate.MovingWall_01_Rotate_C"))
  (for _array_element _outactors
    (Class|BPIInteraction|BpiDaylight(Message) _array_element (Variables|Default|GetDaytime))))